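; BP_Starter_explain is the excavator tutorial's starter, which plays a key sequence and completes the tutorial's starter-click step.
; All four direction events share one path that plays the sequence and waits a fixed delay.
; If its parent actor is an Excavator_Tutorial, it then finishes the behavior tree task handed in through setBT as successful, provided that task is BTTask_Tutorial_Starter_Click.
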(event Custom|set%20BT
  (params (BT :type BT%20Task%20Tutorial%20Starter%20Click%20Object%20Reference))
  (Variables|Default|SetBT BT))

(event EventBeginPlay)

(event Collision|EventActorBeginOverlap
  (params (OtherActor :type Actor%20Object%20Reference)))

(event EventTick
  (params (DeltaSeconds :type Float%20%28single-precision%29)))

(event EventRight
  (params (BT :type Object%20Object%20Reference))
  (Class|ActorSequenceComponent|PlaySequence (Variables|Default|GetKeySequence))
  (Utilities|FlowControl|Delay 6.0)
  (Utilities|Casting|CastToExcavator_Tutorial (Actor|GetParentActor))
  (bind _asbttask_tutorial_starter_click (Utilities|Casting|CastToBTTask_Tutorial_Starter_Click (Variables|Default|GetBT)))
  (AI|BehaviorTree|FinishExecute _asbttask_tutorial_starter_click true))

(event EventUp
  (params (BT :type Object%20Object%20Reference))
  (Class|ActorSequenceComponent|PlaySequence (Variables|Default|GetKeySequence))
  (Utilities|FlowControl|Delay 6.0)
  (Utilities|Casting|CastToExcavator_Tutorial (Actor|GetParentActor))
  (bind _asbttask_tutorial_starter_click (Utilities|Casting|CastToBTTask_Tutorial_Starter_Click (Variables|Default|GetBT)))
  (AI|BehaviorTree|FinishExecute _asbttask_tutorial_starter_click true))

(event EventDown
  (params (BT :type Object%20Object%20Reference))
  (Class|ActorSequenceComponent|PlaySequence (Variables|Default|GetKeySequence))
  (Utilities|FlowControl|Delay 6.0)
  (Utilities|Casting|CastToExcavator_Tutorial (Actor|GetParentActor))
  (bind _asbttask_tutorial_starter_click (Utilities|Casting|CastToBTTask_Tutorial_Starter_Click (Variables|Default|GetBT)))
  (AI|BehaviorTree|FinishExecute _asbttask_tutorial_starter_click true))

(event EventLeft
  (params (BT :type Object%20Object%20Reference))
  (Class|ActorSequenceComponent|PlaySequence (Variables|Default|GetKeySequence))
  (Utilities|FlowControl|Delay 6.0)
  (Utilities|Casting|CastToExcavator_Tutorial (Actor|GetParentActor))
  (bind _asbttask_tutorial_starter_click (Utilities|Casting|CastToBTTask_Tutorial_Starter_Click (Variables|Default|GetBT)))
  (AI|BehaviorTree|FinishExecute _asbttask_tutorial_starter_click true))

(fn ConstructionScript)