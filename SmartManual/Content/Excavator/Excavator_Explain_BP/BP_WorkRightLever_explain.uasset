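; Right work lever of the excavator, used for guided explanation and tutorial practice of arm and bucket control.
; Directional events play level sequences and call arm up/down or bucket bend/bloom on the parent Explain or Simulation excavator.
; Explain runs a timed demo with Korean captions, hand UI cues and mesh animation, then finishes its behavior tree task.
; In tutorial mode, flagged directions finish their BT tasks and briefly show a "Good" widget.
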(event Custom|CustomEvent
  ;[0.15 0.15 0.15 0.5] 이벤트 바인딩
  (Default|CallOnWorkFinished))

(event EventBeginPlay
  ;[0.15 0.15 0.15 0.5] 이벤트 바인딩
  (Input|EnableInput 0)
  (EventDispatchers|BindEventtoOnFinished (Variables|/Script/ActorSequence.ActorSequenceComponent|GetSequencePlayer (Variables|Default|GetRightSequence)) (delegate Custom|CustomEvent))
  (EventDispatchers|BindEventtoOnFinished (Variables|/Script/ActorSequence.ActorSequenceComponent|GetSequencePlayer (Variables|Default|GetLeftSequence)) (delegate Custom|CustomEvent))
  (EventDispatchers|BindEventtoOnFinished (Variables|/Script/ActorSequence.ActorSequenceComponent|GetSequencePlayer (Variables|Default|GetBackSequence)) (delegate Custom|CustomEvent))
  (EventDispatchers|BindEventtoOnFinished (Variables|/Script/ActorSequence.ActorSequenceComponent|GetSequencePlayer (Variables|Default|GetFrontSequence)) (delegate Custom|CustomEvent)))

(event Collision|EventActorBeginOverlap
  (params (OtherActor :type Actor%20Object%20Reference)))

(event EventExplain
  (params (BT :type Object%20Object%20Reference))
  (bind _maoteste (Variables|Default|GetMAOTESTE))
  (Class|ActorSequenceComponent|PlaySequence (Variables|Default|GetLightSequence))
  (bind _ascamera_pawn (Utilities|Casting|CastToCameraPawn (Game|Player|GetPlayerPawn 0)))
  (Default|UpdateExplain _ascamera_pawn "우측 작업레버 입니다.")
  (Utilities|FlowControl|Delay 6.0)
  (Rendering|SetVisibility _maoteste true false)
  (Components|Animation|PlayAnimation _maoteste "/Game/Hand/RightHand/MAOTESTE_Anim.MAOTESTE_Anim" false)
  (Utilities|FlowControl|Delay 0.2)
  (bind _ascamera_pawn_2 (Utilities|Casting|CastToCameraPawn (Game|Player|GetPlayerPawn 0)))
  (Default|UpdateExplain _ascamera_pawn_2 "오른쪽 작업 레버를 뒤로 당기면 암이 내려갑니다.")
  (bind _asexcavator_explain (Utilities|Casting|CastToExcavator_Explain (Actor|GetParentActor)))
  (Default|WorkRightLeverDown (Variables|/Game/Excavator/Excavator_Explain.Excavator_Explain_C|GetHandUI _asexcavator_explain))
  (Utilities|FlowControl|Delay 3.0)
  (CallFunction|PlayBackSequence)
  (Utilities|FlowControl|Delay 2.0)
  (Default|UpdateExplain _ascamera_pawn_2 "오른쪽 작업 레버를 앞으로 당기면 암이 올라갑니다.")
  (Default|WorkRightLeverUp (Variables|/Game/Excavator/Excavator_Explain.Excavator_Explain_C|GetHandUI _asexcavator_explain))
  (Utilities|FlowControl|Delay 3.0)
  (CallFunction|PlayFrontSequence)
  (Utilities|FlowControl|Delay 2.0)
  (Default|UpdateExplain _ascamera_pawn_2 "오른쪽 작업 레버를 오른쪽으로 당기면 버킷이 구부려집니다.")
  (Default|WorkRightLeverRight (Variables|/Game/Excavator/Excavator_Explain.Excavator_Explain_C|GetHandUI _asexcavator_explain))
  (Utilities|FlowControl|Delay 3.0)
  (CallFunction|PlayRightSequence)
  (Utilities|FlowControl|Delay 2.0)
  (Default|UpdateExplain _ascamera_pawn_2 "오른쪽 작업 레버를왼쪽으로 당기면 버킷이 펴집니다.")
  (Default|WorkRightLeverLeft (Variables|/Game/Excavator/Excavator_Explain.Excavator_Explain_C|GetHandUI _asexcavator_explain))
  (Utilities|FlowControl|Delay 3.0)
  (CallFunction|PlayLeftSequence)
  (Utilities|FlowControl|Delay 2.0)
  (bind _asbttask_explain_work_right_lever (Utilities|Casting|CastToBTTask_Explain_WorkRightLever BT))
  (AI|BehaviorTree|FinishExecute _asbttask_explain_work_right_lever true)
  (Rendering|SetVisibility (Variables|Default|GetMAOTESTE) false false))

(event EventTick
  (params (DeltaSeconds :type Float%20%28single-precision%29)))

(event EventLeft
  (params (BT :type Object%20Object%20Reference))
  (CallFunction|PlayLeftSequence)
  (Utilities|FlowControl|Delay 2.0)
  (if (Variables|Default|GetTutorial?)
    (if (Variables|Default|GetTutorial%20Left?)
      (bind _asbttask_explain_work_right_lever_left (Utilities|Casting|CastToBTTask_Explain_WorkRightLever_Left (Variables|Default|GetBT)))
      (AI|BehaviorTree|FinishExecute _asbttask_explain_work_right_lever_left true)
      (bind _returnvalue (UserInterface|CreateWidget "/Game/UI/WBP/WBP_Good.WBP_Good_C" (Game|GetPlayerController 0)))
      (UserInterface|Viewport|AddtoViewport _returnvalue 0)
      (Utilities|FlowControl|Delay 1.0)
      (Widget|RemovefromParent _returnvalue))))

(event EventRight
  (params (BT :type Object%20Object%20Reference))
  (CallFunction|PlayRightSequence)
  (Utilities|FlowControl|Delay 2.0)
  (if (Variables|Default|GetTutorial?)
    (if (Variables|Default|GetTutorial%20Right?)
      (bind _asbttask_explain_work_right_lever_right (Utilities|Casting|CastToBTTask_Explain_WorkRightLever_Right (Variables|Default|GetBT)))
      (AI|BehaviorTree|FinishExecute _asbttask_explain_work_right_lever_right true)
      (bind _returnvalue (UserInterface|CreateWidget "/Game/UI/WBP/WBP_Good.WBP_Good_C" (Game|GetPlayerController 0)))
      (UserInterface|Viewport|AddtoViewport _returnvalue 0)
      (Utilities|FlowControl|Delay 1.0)
      (Widget|RemovefromParent _returnvalue))))

(event EventUp
  (params (BT :type Object%20Object%20Reference))
  (CallFunction|PlayBackSequence)
  (Utilities|FlowControl|Delay 2.0)
  (if (Variables|Default|GetTutorial?)
    (if (Variables|Default|GetTutorial%20Back?)
      (bind _asbttask_explain_work_right_lever_back (Utilities|Casting|CastToBTTask_Explain_WorkRightLever_Back (Variables|Default|GetBT)))
      (AI|BehaviorTree|FinishExecute _asbttask_explain_work_right_lever_back true)
      (bind _returnvalue (UserInterface|CreateWidget "/Game/UI/WBP/WBP_Good.WBP_Good_C" (Game|GetPlayerController 0)))
      (UserInterface|Viewport|AddtoViewport _returnvalue 0)
      (Utilities|FlowControl|Delay 1.0)
      (Widget|RemovefromParent _returnvalue))))

(event EventDown
  (params (BT :type Object%20Object%20Reference))
  (CallFunction|PlayFrontSequence)
  (Utilities|FlowControl|Delay 2.0)
  (if (Variables|Default|GetTutorial?)
    (if (Variables|Default|GetTutorial%20Front?)
      (bind _asbttask_explain_work_right_lever_front (Utilities|Casting|CastToBTTask_Explain_WorkRightLever_Front (Variables|Default|GetBT)))
      (AI|BehaviorTree|FinishExecute _asbttask_explain_work_right_lever_front true)
      (bind _returnvalue (UserInterface|CreateWidget "/Game/UI/WBP/WBP_Good.WBP_Good_C" (Game|GetPlayerController 0)))
      (UserInterface|Viewport|AddtoViewport _returnvalue 0)
      (Utilities|FlowControl|Delay 1.0)
      (Widget|RemovefromParent _returnvalue))))

(event EventTutorial
  (params (BT :type Object%20Object%20Reference))
  (Variables|Default|SetBT BT))

(fn ConstructionScript)

(fn PlayBackSequence
  (bind _returnvalue (Actor|GetParentActor))
  (Class|ActorSequenceComponent|PlaySequence (Variables|Default|GetBackSequence))
  (bind _asexcavator_explain (Utilities|Casting|CastToExcavator_Explain _returnvalue)
    (:then
      (Default|ArmDown _asexcavator_explain))
    (:CastFailed
      (bind _asexcavator_simulation (Utilities|Casting|CastToExcavator_Simulation _returnvalue))
      (Default|ArmDown _asexcavator_simulation))))

(fn PlayFrontSequence
  (bind _returnvalue (Actor|GetParentActor))
  (Class|ActorSequenceComponent|PlaySequence (Variables|Default|GetFrontSequence))
  (bind _asexcavator_explain (Utilities|Casting|CastToExcavator_Explain _returnvalue)
    (:then
      (Default|ArmUp _asexcavator_explain))
    (:CastFailed
      (bind _asexcavator_simulation (Utilities|Casting|CastToExcavator_Simulation _returnvalue))
      (Default|ArmUp _asexcavator_simulation))))

(fn PlayLeftSequence
  (bind _returnvalue (Actor|GetParentActor))
  (Class|ActorSequenceComponent|PlaySequence (Variables|Default|GetLeftSequence))
  (bind _asexcavator_explain (Utilities|Casting|CastToExcavator_Explain _returnvalue)
    (:then
      (Default|BasketBloom _asexcavator_explain))
    (:CastFailed
      (bind _asexcavator_simulation (Utilities|Casting|CastToExcavator_Simulation _returnvalue))
      (Default|BasketBloom _asexcavator_simulation))))

(fn PlayRightSequence
  (bind _returnvalue (Actor|GetParentActor))
  (Class|ActorSequenceComponent|PlaySequence (Variables|Default|GetRightSequence))
  (bind _asexcavator_explain (Utilities|Casting|CastToExcavator_Explain _returnvalue)
    (:then
      (Default|BasketBend _asexcavator_explain))
    (:CastFailed
      (bind _asexcavator_simulation (Utilities|Casting|CastToExcavator_Simulation _returnvalue))
      (Default|BasketBend _asexcavator_simulation))))