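; Excavator left work lever actor that demonstrates its controls in a guided explanation run by a behavior tree task.
; Explain shows Korean captions on the CameraPawn while timed steps play four directional level sequences and drive the parent Excavator_Explain's boom and swing.
; It then calls FinishExecute on the passed BTTask_Explain_WorkLeftLever.
; Finished sequences fire OnWorkFinished; directional input events and Tutorial only print debug strings.
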(event Custom|CustomEvent
  ;[0.15 0.15 0.15 0.5] 이벤트 바인딩
  (Default|CallOnWorkFinished))

(event EventBeginPlay
  ;[0.15 0.15 0.15 0.5] 이벤트 바인딩
  (Input|EnableInput 0)
  (EventDispatchers|BindEventtoOnFinished (Variables|/Script/ActorSequence.ActorSequenceComponent|GetSequencePlayer (Variables|Default|GetRightSequence)) (delegate Custom|CustomEvent))
  (EventDispatchers|BindEventtoOnFinished (Variables|/Script/ActorSequence.ActorSequenceComponent|GetSequencePlayer (Variables|Default|GetLeftSequence)) (delegate Custom|CustomEvent))
  (EventDispatchers|BindEventtoOnFinished (Variables|/Script/ActorSequence.ActorSequenceComponent|GetSequencePlayer (Variables|Default|GetBackSequence)) (delegate Custom|CustomEvent))
  (EventDispatchers|BindEventtoOnFinished (Variables|/Script/ActorSequence.ActorSequenceComponent|GetSequencePlayer (Variables|Default|GetFrontSequence)) (delegate Custom|CustomEvent)))

(event Collision|EventActorBeginOverlap
  (params (OtherActor :type Actor%20Object%20Reference)))

(event EventExplain
  (params (BT :type Object%20Object%20Reference))
  (bind _ascamera_pawn (Utilities|Casting|CastToCameraPawn (Game|Player|GetPlayerPawn 0)))
  (Default|UpdateExplain _ascamera_pawn "왼쪽 작업 레버를 뒤로 당기면 붐이 내려갑니다.")
  (CallFunction|PlayBackSequence)
  (Utilities|FlowControl|Delay 2.0)
  (Default|UpdateExplain _ascamera_pawn "왼쪽 작업 레버를 앞으로 당기면 붐이 올라갑니다.")
  (CallFunction|PlayFrontSequence)
  (Utilities|FlowControl|Delay 2.0)
  (Default|UpdateExplain _ascamera_pawn "왼쪽 작업 레버를 오른쪽으로 당기면 본체가 우회전 합 니다.")
  (CallFunction|PlayRightSequence)
  (Utilities|FlowControl|Delay 2.0)
  (bind _asexcavator_explain (Utilities|Casting|CastToExcavator_Explain (Actor|GetParentActor)))
  (Variables|/Game/Excavator/Excavator_Explain.Excavator_Explain_C|SetTurnRight? _asexcavator_explain false)
  (Default|UpdateExplain _ascamera_pawn "왼쪽 작업 레버를 왼쪽으로 당기면 본체가 좌회전 합 니다.")
  (CallFunction|PlayLeftSequence)
  (Utilities|FlowControl|Delay 2.0)
  (Variables|/Game/Excavator/Excavator_Explain.Excavator_Explain_C|SetTurnLeft? _asexcavator_explain false)
  (bind _asbttask_explain_work_left_lever (Utilities|Casting|CastToBTTask_Explain_WorkLeftLever BT))
  (AI|BehaviorTree|FinishExecute _asbttask_explain_work_left_lever true))

(event EventTick
  (params (DeltaSeconds :type Float%20%28single-precision%29)))

(event EventLeft
  (Development|PrintString "WorkLeftLever : 좌"))

(event EventRight
  (Development|PrintString "WorkLeftLever : 우"))

(event EventUp
  (Development|PrintString "WorkLeftLever : 상"))

(event EventDown
  (Development|PrintString "WorkLeftLever : 하"))

(event EventTutorial
  (params (BT :type Object%20Object%20Reference))
  (Development|PrintString "WorkLeftLever  tutorial"))

(fn ConstructionScript)

(fn PlayBackSequence
  (Class|ActorSequenceComponent|PlaySequence (Variables|Default|GetBackSequence))
  (bind _asexcavator_explain (Utilities|Casting|CastToExcavator_Explain (Actor|GetParentActor)))
  (Default|BoomDown _asexcavator_explain))

(fn PlayFrontSequence
  (Class|ActorSequenceComponent|PlaySequence (Variables|Default|GetFrontSequence))
  (bind _asexcavator_explain (Utilities|Casting|CastToExcavator_Explain (Actor|GetParentActor)))
  (Default|BoomUp _asexcavator_explain))

(fn PlayLeftSequence
  (Class|ActorSequenceComponent|PlaySequence (Variables|Default|GetLeftSequence))
  (bind _asexcavator_explain (Utilities|Casting|CastToExcavator_Explain (Actor|GetParentActor)))
  (Variables|/Game/Excavator/Excavator_Explain.Excavator_Explain_C|SetTurnLeft? _asexcavator_explain true))

(fn PlayRightSequence
  (Class|ActorSequenceComponent|PlaySequence (Variables|Default|GetRightSequence))
  (bind _asexcavator_explain (Utilities|Casting|CastToExcavator_Explain (Actor|GetParentActor)))
  (Variables|/Game/Excavator/Excavator_Explain.Excavator_Explain_C|SetTurnRight? _asexcavator_explain true))