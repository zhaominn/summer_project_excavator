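; Excavator right work lever actor that demonstrates arm and bucket control through four directional sequences.
; Explain steps through Korean captions on the CameraPawn, playing each sequence at two-second intervals, then finishes the passed behavior tree task, cast to BTTask_Explain_WorkLeftLever despite this being the right lever.
; Each sequence's finish fires OnWorkFinished.
; BeginPlay enables input, but directional events only print debug text.
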(event Custom|CustomEvent
  ;[0.15 0.15 0.15 0.5] 이벤트 바인딩
  (Default|CallOnWorkFinished))

(event EventBeginPlay
  ;[0.15 0.15 0.15 0.5] 이벤트 바인딩
  (Input|EnableInput 0)
  (EventDispatchers|BindEventtoOnFinished (Variables|/Script/ActorSequence.ActorSequenceComponent|GetSequencePlayer (Variables|Default|GetRightSequence)) (delegate Custom|CustomEvent))
  (EventDispatchers|BindEventtoOnFinished (Variables|/Script/ActorSequence.ActorSequenceComponent|GetSequencePlayer (Variables|Default|GetLeftSequence)) (delegate Custom|CustomEvent))
  (EventDispatchers|BindEventtoOnFinished (Variables|/Script/ActorSequence.ActorSequenceComponent|GetSequencePlayer (Variables|Default|GetFrontSequence)) (delegate Custom|CustomEvent))
  (EventDispatchers|BindEventtoOnFinished (Variables|/Script/ActorSequence.ActorSequenceComponent|GetSequencePlayer (Variables|Default|GetBackSequence)) (delegate Custom|CustomEvent)))

(event Collision|EventActorBeginOverlap
  (params (OtherActor :type Actor%20Object%20Reference)))

(event EventExplain
  (params (BT :type Object%20Object%20Reference))
  (bind _ascamera_pawn (Utilities|Casting|CastToCameraPawn (Game|Player|GetPlayerPawn 0)))
  (Default|UpdateExplain _ascamera_pawn "오른쪽 작업 레버를 뒤로 당기면 암이 내려갑니다.")
  (CallFunction|PlayBackSequence)
  (Utilities|FlowControl|Delay 2.0)
  (Default|UpdateExplain _ascamera_pawn "오른쪽 작업 레버를 앞으로 당기면 암이 올라갑니다.")
  (CallFunction|PlayFrontSequence)
  (Utilities|FlowControl|Delay 2.0)
  (Default|UpdateExplain _ascamera_pawn "오른쪽 작업 레버를 오른쪽으로 당기면 버킷이 구부려집니다.")
  (CallFunction|PlayRightSequence)
  (Utilities|FlowControl|Delay 2.0)
  (Default|UpdateExplain _ascamera_pawn "오른쪽 작업 레버를왼쪽으로 당기면 버킷이 펴집니다.")
  (CallFunction|PlayLeftSequence)
  (Utilities|FlowControl|Delay 2.0)
  (bind _asbttask_explain_work_left_lever (Utilities|Casting|CastToBTTask_Explain_WorkLeftLever BT))
  (AI|BehaviorTree|FinishExecute _asbttask_explain_work_left_lever true))

(event EventTick
  (params (DeltaSeconds :type Float%20%28single-precision%29)))

(event EventLeft
  (Development|PrintString "WorkRightLever : 좌"))

(event EventRight
  (Development|PrintString "WorkRightLever : 우"))

(event EventUp
  (Development|PrintString "WorkRightLever : 상"))

(event EventDown
  (Development|PrintString "WorkRightLever : 하"))

(fn ConstructionScript)

(fn PlayBackSequence
  (Class|ActorSequenceComponent|PlaySequence (Variables|Default|GetBackSequence)))

(fn PlayFrontSequence
  (Class|ActorSequenceComponent|PlaySequence (Variables|Default|GetFrontSequence)))

(fn PlayLeftSequence
  (Class|ActorSequenceComponent|PlaySequence (Variables|Default|GetLeftSequence)))

(fn PlayRightSequence
  (Class|ActorSequenceComponent|PlaySequence (Variables|Default|GetRightSequence)))