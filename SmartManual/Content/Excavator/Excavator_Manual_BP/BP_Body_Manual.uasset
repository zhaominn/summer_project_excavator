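; Excavator manual part actor for the operator's cab (운전석), which presents an explanation of that part when clicked.
; On BeginPlay it writes the part name into its WBP_Object label, whose visibility Tick toggles to show only at level index 0 in BP_Instance.
; A click blends the player camera to this actor, then after a delay sets the cab's Korean description on the WBP_BTN_Manual widget.
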(event OnClicked(Widget_)
  (params (TouchedComponent :type Primitive%20Component%20Object%20Reference) (ButtonPressed :type Key%20Structure :default "None"))
  (Game|Player|SetViewTargetwithBlend (Game|GetPlayerController 0) self 1.0 "VTBlend_Linear" 0.0 false)
  (bind _foundwidgets (Widget|GetAllWidgetsOfClass "/Game/UI/Manual/WBP_BTN_Manual.WBP_BTN_Manual_C" true))
  (Utilities|FlowControl|Delay 1.0)
  (Variables|/Game/UI/Manual/WBP_BTN_Manual.WBP_BTN_Manual_C|SetManual_Text (Utilities|Array|Get(acopy) _foundwidgets) "운전석은 조종사가 앉아 레버와 페달을 조작해 포크레인을 움직이고 작업을 제어하는 공간입니다."))

(event EventBeginPlay
  (bind _aswbp_object (Utilities|Casting|CastToWBP_Object (UserInterface|GetUserWidgetObject (Variables|Default|GetWidget_))))
  (Variables|/Game/UI/Manual/WBP_Object.WBP_Object_C|Setobject _aswbp_object "운전석"))

(event Collision|EventActorBeginOverlap
  (params (OtherActor :type Actor%20Object%20Reference)))

(event EventTick
  (params (DeltaSeconds :type Float%20%28single-precision%29))
  (bind _widget_ (Variables|Default|GetWidget_))
  (bind _asbp_instance (Utilities|Casting|CastToBP_Instance (Game|GetGameInstance)))
  (if (== 0 (Variables|/Game/Maps/manual/BP_Instance.BP_Instance_C|GetCurrentLevelIndex _asbp_instance))
    (Rendering|SetVisibility _widget_ true false)
    (else
      (Rendering|SetVisibility _widget_ false false))))

(fn ConstructionScript)