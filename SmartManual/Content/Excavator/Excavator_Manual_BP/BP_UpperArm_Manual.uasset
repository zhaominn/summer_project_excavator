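; Manually controlled excavator upper arm that exposes playback of preset motions for the arm, boom and basket.
; Six functions each call PlaySequence on their own sequence reference, covering arm up and down, boom up and down, and basket bend and bloom.
; It holds no input, event or blending logic, so playback depends on these functions being called.
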(event EventBeginPlay)

(event Collision|EventActorBeginOverlap
  (params (OtherActor :type Actor%20Object%20Reference)))

(event EventTick
  (params (DeltaSeconds :type Float%20%28single-precision%29)))

(fn ConstructionScript)

(fn PlayArmDown
  (Class|ActorSequenceComponent|PlaySequence (Variables|Default|GetArm%20Down)))

(fn PlayArmUp
  (Class|ActorSequenceComponent|PlaySequence (Variables|Default|GetArm%20Up)))

(fn PlayBoomDown
  (Class|ActorSequenceComponent|PlaySequence (Variables|Default|GetBoom%20Down)))

(fn PlayBoomUp
  (Class|ActorSequenceComponent|PlaySequence (Variables|Default|GetBoom%20Up)))

(fn PlayBasketBend
  (Class|ActorSequenceComponent|PlaySequence (Variables|Default|GetBasket%20Bend)))

(fn PlayBasketBloom
  (Class|ActorSequenceComponent|PlaySequence (Variables|Default|GetBasket%20Bloom)))