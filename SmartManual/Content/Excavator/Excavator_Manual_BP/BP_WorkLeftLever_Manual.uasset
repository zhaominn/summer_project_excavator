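; Manual excavator left work lever that animates its movement and drives boom and turning on the parent excavator.
; Four functions, one per direction, each play their sequence, then cast the parent actor to Excavator_Explain, falling back to Excavator_Simulation.
; Front and back call BoomUp and BoomDown, while left and right only set TurnLeft or TurnRight to true, with no reset here.
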(fn ConstructionScript)

(fn PlayBackSequence
  (bind _returnvalue (Actor|GetParentActor))
  (Class|ActorSequenceComponent|PlaySequence (Variables|Default|GetBackSequence))
  (bind _asexcavator_explain (Utilities|Casting|CastToExcavator_Explain _returnvalue)
    (:then
      (Default|BoomDown _asexcavator_explain))
    (:CastFailed
      (bind _asexcavator_simulation (Utilities|Casting|CastToExcavator_Simulation _returnvalue))
      (Default|BoomDown _asexcavator_simulation))))

(fn PlayFrontSequence
  (bind _returnvalue (Actor|GetParentActor))
  (Class|ActorSequenceComponent|PlaySequence (Variables|Default|GetFrontSequence))
  (bind _asexcavator_explain (Utilities|Casting|CastToExcavator_Explain _returnvalue)
    (:then
      (Default|BoomUp _asexcavator_explain))
    (:CastFailed
      (bind _asexcavator_simulation (Utilities|Casting|CastToExcavator_Simulation _returnvalue))
      (Default|BoomUp _asexcavator_simulation))))

(fn PlayLeftSequence
  (bind _returnvalue (Actor|GetParentActor))
  (Class|ActorSequenceComponent|PlaySequence (Variables|Default|GetLeftSequence))
  (bind _asexcavator_explain (Utilities|Casting|CastToExcavator_Explain _returnvalue)
    (:then
      (Variables|/Game/Excavator/Excavator_Explain.Excavator_Explain_C|SetTurnLeft? _asexcavator_explain true))
    (:CastFailed
      (bind _asexcavator_simulation (Utilities|Casting|CastToExcavator_Simulation _returnvalue))
      (Variables|/Game/Excavator/Excavator_Simulation.Excavator_Simulation_C|SetTurnLeft? _asexcavator_simulation true))))

(fn PlayRightSequence
  (bind _returnvalue (Actor|GetParentActor))
  (Class|ActorSequenceComponent|PlaySequence (Variables|Default|GetRightSequence))
  (bind _asexcavator_explain (Utilities|Casting|CastToExcavator_Explain _returnvalue)
    (:then
      (Variables|/Game/Excavator/Excavator_Explain.Excavator_Explain_C|SetTurnRight? _asexcavator_explain true))
    (:CastFailed
      (bind _asexcavator_simulation (Utilities|Casting|CastToExcavator_Simulation _returnvalue))
      (Variables|/Game/Excavator/Excavator_Simulation.Excavator_Simulation_C|SetTurnRight? _asexcavator_simulation true))))