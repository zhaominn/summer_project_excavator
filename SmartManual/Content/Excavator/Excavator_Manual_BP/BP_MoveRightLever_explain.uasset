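; Excavator right travel lever actor that demonstrates reverse and forward driving in a guided explanation.
; Explain shows pawn text, plays back then front sequences with delays, clears parent drive flags and finishes the calling behavior tree task.
; PlayBacksequence flags either Explain or Simulation parents, while PlayFrontSequence flags only Simulation, leaving its Explain branch unwired.
; Up/Down forward messages to the parent; finished sequences call OnWorkFinished.
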(event Custom|CustomEvent
  ;[0.15 0.15 0.15 0.5] 이벤트 바인딩
  (Default|CallOnWorkFinished))

(event EventBeginPlay
  ;[0.15 0.15 0.15 0.5] 이벤트 바인딩
  (Input|EnableInput 0)
  (EventDispatchers|BindEventtoOnFinished (Variables|/Script/ActorSequence.ActorSequenceComponent|GetSequencePlayer (Variables|Default|GetFrontSequence)) (delegate Custom|CustomEvent))
  (EventDispatchers|BindEventtoOnFinished (Variables|/Script/ActorSequence.ActorSequenceComponent|GetSequencePlayer (Variables|Default|GetBackSequence)) (delegate Custom|CustomEvent)))

(event Collision|EventActorBeginOverlap
  (params (OtherActor :type Actor%20Object%20Reference)))

(event EventTick
  (params (DeltaSeconds :type Float%20%28single-precision%29)))

(event EventExplain
  (params (BT :type Object%20Object%20Reference))
  (bind _ascamera_pawn (Utilities|Casting|CastToCameraPawn (Game|Player|GetPlayerPawn 0)))
  (Default|UpdateExplain _ascamera_pawn "오른쪽 주행 레버를 뒤로 당기면 후진합니다.")
  (CallFunction|PlayBacksequence)
  (Utilities|FlowControl|Delay 2.0)
  (bind _asexcavator_explain (Utilities|Casting|CastToExcavator_Explain (Actor|GetParentActor)))
  (Variables|/Game/Excavator/Excavator_Explain.Excavator_Explain_C|SetGoBack_Right? _asexcavator_explain false)
  (Default|UpdateExplain _ascamera_pawn "오른쪽 주행 레버를 뒤로 당기면 후진합니다.")
  (CallFunction|PlayFrontSequence)
  (Utilities|FlowControl|Delay 2.0)
  (Variables|/Game/Excavator/Excavator_Explain.Excavator_Explain_C|SetGoStraight_Right? _asexcavator_explain false)
  (bind _asbttask_explain_move_right_lever (Utilities|Casting|CastToBTTask_Explain_MoveRightLever BT))
  (AI|BehaviorTree|FinishExecute _asbttask_explain_move_right_lever true))

(event EventUp
  (params (BT :type Object%20Object%20Reference))
  (bind _returnvalue (Actor|GetParentActor))
  (Class|ComponentInterface|Up(Message) _returnvalue _returnvalue))

(event EventDown
  (params (BT :type Object%20Object%20Reference))
  (bind _returnvalue (Actor|GetParentActor))
  (Class|ComponentInterface|Down(Message) _returnvalue _returnvalue))

(fn ConstructionScript)

(fn PlayFrontSequence
  (Class|ActorSequenceComponent|PlaySequence (Variables|Default|GetFrontSequence))
  (bind _asexcavator_simulation (Utilities|Casting|CastToExcavator_Simulation (Actor|GetParentActor)))
  (Variables|/Game/Excavator/Excavator_Simulation.Excavator_Simulation_C|SetGoStraight_Right? _asexcavator_simulation true))

(fn PlayBacksequence
  (bind _returnvalue (Actor|GetParentActor))
  (Class|ActorSequenceComponent|PlaySequence (Variables|Default|GetBackSequence))
  (bind _asexcavator_explain (Utilities|Casting|CastToExcavator_Explain _returnvalue)
    (:then
      (Variables|/Game/Excavator/Excavator_Explain.Excavator_Explain_C|SetGoBack_Right? _asexcavator_explain true))
    (:CastFailed
      (bind _asexcavator_simulation (Utilities|Casting|CastToExcavator_Simulation _returnvalue))
      (Variables|/Game/Excavator/Excavator_Simulation.Excavator_Simulation_C|SetGoBack_Right? _asexcavator_simulation true))))