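; BP_LowArm_Manual is an excavator manual actor for the arm part, the link that moves the bucket.
; On BeginPlay it sets its ArmWidget label to the Korean word for arm.
; Clicking Arm_widget blends the player's view to this actor over one second.
; After a matching delay, it writes the arm's Korean explanation into the first top-level WBP_BTN_Manual widget found.
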(event OnClicked(arm_widget)
  (params (TouchedComponent :type Primitive%20Component%20Object%20Reference) (ButtonPressed :type Key%20Structure :default "None"))
  (Game|Player|SetViewTargetwithBlend (Game|GetPlayerController 0) self 1.0 "VTBlend_Linear" 0.0 false)
  (bind _foundwidgets (Widget|GetAllWidgetsOfClass "/Game/UI/Manual/WBP_BTN_Manual.WBP_BTN_Manual_C" true))
  (Utilities|FlowControl|Delay 1.0)
  (Variables|/Game/UI/Manual/WBP_BTN_Manual.WBP_BTN_Manual_C|SetManual_Text (Utilities|Array|Get(acopy) _foundwidgets) "암(Arm)은 버킷을 움직여 땅을 파고 자재를 들어 올릴 수 있게 연결해주는 팔 역할을 합니다."))

(event EventBeginPlay
  (bind _aswbp_object (Utilities|Casting|CastToWBP_Object (UserInterface|GetUserWidgetObject (Variables|Default|Getarm_widget))))
  (Variables|/Game/UI/Manual/WBP_Object.WBP_Object_C|Setobject _aswbp_object "암"))

(event Collision|EventActorBeginOverlap
  (params (OtherActor :type Actor%20Object%20Reference)))

(event EventTick
  (params (DeltaSeconds :type Float%20%28single-precision%29)))

(fn ConstructionScript)