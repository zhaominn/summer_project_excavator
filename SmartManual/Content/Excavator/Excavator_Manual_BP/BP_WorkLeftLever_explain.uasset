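; Left work lever of the excavator that plays directional sequences to raise or lower the boom or swing the body left or right.
; Each movement drives the parent Excavator_Explain, falling back to Excavator_Simulation.
; Explain runs a timed demo with captions and hand-UI hints, then finishes its behavior tree task.
; Left, Right, Up and Down play single moves, completing matching tutorial tasks with a brief WBP_Good popup when flagged.
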(event Custom|CustomEvent
  ;[0.15 0.15 0.15 0.5] 이벤트 바인딩
  (Default|CallOnWorkFinished))

(event EventBeginPlay
  ;[0.15 0.15 0.15 0.5] 이벤트 바인딩
  (Input|EnableInput 0)
  (EventDispatchers|BindEventtoOnFinished (Variables|/Script/ActorSequence.ActorSequenceComponent|GetSequencePlayer (Variables|Default|GetRightSequence)) (delegate Custom|CustomEvent))
  (EventDispatchers|BindEventtoOnFinished (Variables|/Script/ActorSequence.ActorSequenceComponent|GetSequencePlayer (Variables|Default|GetLeftSequence)) (delegate Custom|CustomEvent))
  (EventDispatchers|BindEventtoOnFinished (Variables|/Script/ActorSequence.ActorSequenceComponent|GetSequencePlayer (Variables|Default|GetBackSequence)) (delegate Custom|CustomEvent))
  (EventDispatchers|BindEventtoOnFinished (Variables|/Script/ActorSequence.ActorSequenceComponent|GetSequencePlayer (Variables|Default|GetFrontSequence)) (delegate Custom|CustomEvent)))

(event Collision|EventActorBeginOverlap
  (params (OtherActor :type Actor%20Object%20Reference)))

(event EventExplain
  (params (BT :type Object%20Object%20Reference))
  (bind _ascamera_pawn (Utilities|Casting|CastToCameraPawn (Game|Player|GetPlayerPawn 0)))
  (Default|UpdateExplain _ascamera_pawn "왼쪽 작업 레버를 뒤로 당기면 붐이 내려갑니다.")
  (bind _asexcavator_explain (Utilities|Casting|CastToExcavator_Explain (Actor|GetParentActor)))
  (Default|WorkLeftLeverDown (Variables|/Game/Excavator/Excavator_Explain.Excavator_Explain_C|GetHandUI _asexcavator_explain))
  (Utilities|FlowControl|Delay 3.0)
  (CallFunction|PlayBackSequence)
  (Utilities|FlowControl|Delay 2.0)
  (Default|UpdateExplain _ascamera_pawn "왼쪽 작업 레버를 앞으로 당기면 붐이 올라갑니다.")
  (Default|WorkLeftLeverUp (Variables|/Game/Excavator/Excavator_Explain.Excavator_Explain_C|GetHandUI _asexcavator_explain))
  (Utilities|FlowControl|Delay 3.0)
  (CallFunction|PlayFrontSequence)
  (Utilities|FlowControl|Delay 2.0)
  (Default|UpdateExplain _ascamera_pawn "왼쪽 작업 레버를 오른쪽으로 당기면 본체가 우회전 합 니다.")
  (Default|WorkLeftLeverRight (Variables|/Game/Excavator/Excavator_Explain.Excavator_Explain_C|GetHandUI _asexcavator_explain))
  (Utilities|FlowControl|Delay 3.0)
  (CallFunction|PlayRightSequence)
  (Utilities|FlowControl|Delay 2.0)
  (Variables|/Game/Excavator/Excavator_Explain.Excavator_Explain_C|SetTurnRight? _asexcavator_explain false)
  (Default|UpdateExplain _ascamera_pawn "왼쪽 작업 레버를 왼쪽으로 당기면 본체가 좌회전 합 니다.")
  (Default|WorkLeftLeverLeft (Variables|/Game/Excavator/Excavator_Explain.Excavator_Explain_C|GetHandUI _asexcavator_explain))
  (Utilities|FlowControl|Delay 3.0)
  (CallFunction|PlayLeftSequence)
  (Utilities|FlowControl|Delay 2.0)
  (Variables|/Game/Excavator/Excavator_Explain.Excavator_Explain_C|SetTurnLeft? _asexcavator_explain false)
  (bind _asbttask_explain_work_left_lever (Utilities|Casting|CastToBTTask_Explain_WorkLeftLever BT))
  (AI|BehaviorTree|FinishExecute _asbttask_explain_work_left_lever true))

(event EventTick
  (params (DeltaSeconds :type Float%20%28single-precision%29)))

(event EventRight
  (params (BT :type Object%20Object%20Reference))
  (bind _returnvalue (Actor|GetParentActor))
  (CallFunction|PlayRightSequence)
  (Utilities|FlowControl|Delay 2.0)
  (bind _asexcavator_explain (Utilities|Casting|CastToExcavator_Explain _returnvalue)
    (:then
      (Variables|/Game/Excavator/Excavator_Explain.Excavator_Explain_C|SetTurnRight? _asexcavator_explain false)
      (if (Variables|Default|GetTutorial?)
        (if (Variables|Default|GetTutorial%20Right?)
          (bind _asbttask_explain_work_left_lever_right (Utilities|Casting|CastToBTTask_Explain_WorkLeftLever_Right (Variables|Default|GetBT)))
          (AI|BehaviorTree|FinishExecute _asbttask_explain_work_left_lever_right true)
          (bind _returnvalue_2 (UserInterface|CreateWidget "/Game/UI/WBP/WBP_Good.WBP_Good_C" (Game|GetPlayerController 0)))
          (UserInterface|Viewport|AddtoViewport _returnvalue_2 0)
          (Utilities|FlowControl|Delay 1.0)
          (Widget|RemovefromParent _returnvalue_2))))
    (:CastFailed
      (bind _asexcavator_simulation (Utilities|Casting|CastToExcavator_Simulation _returnvalue))
      (Variables|/Game/Excavator/Excavator_Simulation.Excavator_Simulation_C|SetTurnRight? _asexcavator_simulation false))))

(event EventUp
  (params (BT :type Object%20Object%20Reference))
  (bind _returnvalue (Actor|GetParentActor))
  (CallFunction|PlayBackSequence)
  (Utilities|FlowControl|Delay 2.0)
  (bind _asexcavator_explain (Utilities|Casting|CastToExcavator_Explain _returnvalue)
    (:then
      (Variables|/Game/Excavator/Excavator_Explain.Excavator_Explain_C|SetGoBack_Left? _asexcavator_explain false)
      (if (Variables|Default|GetTutorial?)
        (if (Variables|Default|GetTutorial%20Back?)
          (bind _asbttask_explain_work_left_lever_back (Utilities|Casting|CastToBTTask_Explain_WorkLeftLever_Back (Variables|Default|GetBT)))
          (AI|BehaviorTree|FinishExecute _asbttask_explain_work_left_lever_back true)
          (bind _returnvalue_2 (UserInterface|CreateWidget "/Game/UI/WBP/WBP_Good.WBP_Good_C" (Game|GetPlayerController 0)))
          (UserInterface|Viewport|AddtoViewport _returnvalue_2 0)
          (Utilities|FlowControl|Delay 1.0)
          (Widget|RemovefromParent _returnvalue_2))))
    (:CastFailed
      (bind _asexcavator_simulation (Utilities|Casting|CastToExcavator_Simulation _returnvalue))
      (Variables|/Game/Excavator/Excavator_Simulation.Excavator_Simulation_C|SetGoBack_Left? _asexcavator_simulation false))))

(event EventDown
  (params (BT :type Object%20Object%20Reference))
  (bind _returnvalue (Actor|GetParentActor))
  (CallFunction|PlayFrontSequence)
  (Utilities|FlowControl|Delay 2.0)
  (bind _asexcavator_explain (Utilities|Casting|CastToExcavator_Explain _returnvalue)
    (:then
      (Variables|/Game/Excavator/Excavator_Explain.Excavator_Explain_C|SetGoStraight_Left? _asexcavator_explain false)
      (if (Variables|Default|GetTutorial?)
        (if (Variables|Default|GetTutorial%20Front?)
          (bind _asbttask_explain_work_left_lever_front (Utilities|Casting|CastToBTTask_Explain_WorkLeftLever_Front (Variables|Default|GetBT)))
          (AI|BehaviorTree|FinishExecute _asbttask_explain_work_left_lever_front true)
          (bind _returnvalue_2 (UserInterface|CreateWidget "/Game/UI/WBP/WBP_Good.WBP_Good_C" (Game|GetPlayerController 0)))
          (UserInterface|Viewport|AddtoViewport _returnvalue_2 0)
          (Utilities|FlowControl|Delay 1.0)
          (Widget|RemovefromParent _returnvalue_2))))
    (:CastFailed
      (bind _asexcavator_simulation (Utilities|Casting|CastToExcavator_Simulation _returnvalue))
      (Variables|/Game/Excavator/Excavator_Simulation.Excavator_Simulation_C|SetGoBack_Right? _asexcavator_simulation false))))

(event EventTutorial
  (params (BT :type Object%20Object%20Reference))
  (Variables|Default|SetBT BT))

(event EventLeft
  (params (BT :type Object%20Object%20Reference))
  (bind _returnvalue (Actor|GetParentActor))
  (CallFunction|PlayLeftSequence)
  (Utilities|FlowControl|Delay 2.0)
  (bind _asexcavator_explain (Utilities|Casting|CastToExcavator_Explain _returnvalue)
    (:then
      (Variables|/Game/Excavator/Excavator_Explain.Excavator_Explain_C|SetTurnLeft? _asexcavator_explain false)
      (if (Variables|Default|GetTutorial?)
        (if (Variables|Default|GetTutorial%20Left?)
          (bind _asbttask_explain_work_left_lever_left (Utilities|Casting|CastToBTTask_Explain_WorkLeftLever_Left (Variables|Default|GetBT)))
          (AI|BehaviorTree|FinishExecute _asbttask_explain_work_left_lever_left true)
          (bind _returnvalue_2 (UserInterface|CreateWidget "/Game/UI/WBP/WBP_Good.WBP_Good_C" (Game|GetPlayerController 0)))
          (UserInterface|Viewport|AddtoViewport _returnvalue_2 0)
          (Utilities|FlowControl|Delay 1.0)
          (Widget|RemovefromParent _returnvalue_2))))
    (:CastFailed
      (bind _asexcavator_simulation (Utilities|Casting|CastToExcavator_Simulation _returnvalue))
      (Variables|/Game/Excavator/Excavator_Simulation.Excavator_Simulation_C|SetTurnLeft? _asexcavator_simulation false))))

(fn ConstructionScript)

(fn PlayBackSequence
  (bind _returnvalue (Actor|GetParentActor))
  (Class|ActorSequenceComponent|PlaySequence (Variables|Default|GetBackSequence))
  (bind _asexcavator_explain (Utilities|Casting|CastToExcavator_Explain _returnvalue)
    (:then
      (Default|BoomDown _asexcavator_explain))
    (:CastFailed
      (bind _asexcavator_simulation (Utilities|Casting|CastToExcavator_Simulation _returnvalue))
      (Default|BoomDown _asexcavator_simulation))))

(fn PlayFrontSequence
  (bind _returnvalue (Actor|GetParentActor))
  (Class|ActorSequenceComponent|PlaySequence (Variables|Default|GetFrontSequence))
  (bind _asexcavator_explain (Utilities|Casting|CastToExcavator_Explain _returnvalue)
    (:then
      (Default|BoomUp _asexcavator_explain))
    (:CastFailed
      (bind _asexcavator_simulation (Utilities|Casting|CastToExcavator_Simulation _returnvalue))
      (Default|BoomUp _asexcavator_simulation))))

(fn PlayLeftSequence
  (bind _returnvalue (Actor|GetParentActor))
  (Class|ActorSequenceComponent|PlaySequence (Variables|Default|GetLeftSequence))
  (bind _asexcavator_explain (Utilities|Casting|CastToExcavator_Explain _returnvalue)
    (:then
      (Variables|/Game/Excavator/Excavator_Explain.Excavator_Explain_C|SetTurnLeft? _asexcavator_explain true))
    (:CastFailed
      (bind _asexcavator_simulation (Utilities|Casting|CastToExcavator_Simulation _returnvalue))
      (Variables|/Game/Excavator/Excavator_Simulation.Excavator_Simulation_C|SetTurnLeft? _asexcavator_simulation true))))

(fn PlayRightSequence
  (bind _returnvalue (Actor|GetParentActor))
  (Class|ActorSequenceComponent|PlaySequence (Variables|Default|GetRightSequence))
  (bind _asexcavator_explain (Utilities|Casting|CastToExcavator_Explain _returnvalue)
    (:then
      (Variables|/Game/Excavator/Excavator_Explain.Excavator_Explain_C|SetTurnRight? _asexcavator_explain true))
    (:CastFailed
      (bind _asexcavator_simulation (Utilities|Casting|CastToExcavator_Simulation _returnvalue))
      (Variables|/Game/Excavator/Excavator_Simulation.Excavator_Simulation_C|SetTurnRight? _asexcavator_simulation true))))