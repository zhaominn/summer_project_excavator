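; Bucket actor for the excavator simulation, nested as a child actor under the upper arm.
; Its Collision? event writes a quest index to the QuestNumber blackboard key of the grandparent actor's AI controller, then creates a rock.
; Rocks spawn at the bucket's Arrow component and keep a reference back to the bucket.
; A reset event zeroes the basket, arm and boom pivot rotations on the parent BP_UpperArm.
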(event Custom|create%20Rock
  (bind _returnvalue (Game|SpawnActorfromClass "/Game/Blueprints/BP_Rock.BP_Rock_C" (Math|Transform|MakeTransform (Transformation|GetWorldLocation (Variables|Default|GetArrow)) "0, 0, 0" "1.000000,1.000000,1.000000") "Undefined" "MultiplyWithRoot" 0 0))
  (Variables|/Game/Blueprints/BP_Rock.BP_Rock_C|SetBP_Bascket _returnvalue self))

(event Custom|reset_Arm
  (bind _asbp_upper_arm (Utilities|Casting|CastToBP_UpperArm (Actor|GetParentActor)))
  (Transformation|SetRelativeRotation (Variables|/Game/Excavator/ExcavatorSimulation_BP/BP_UpperArm.BP_UpperArm_C|GetBasket%20Pivot _asbp_upper_arm) "0, 0, 0" false false)
  (Transformation|SetRelativeRotation (Variables|/Game/Excavator/ExcavatorSimulation_BP/BP_UpperArm.BP_UpperArm_C|GetArm%20Pivot _asbp_upper_arm) "0, 0, 0" false false)
  (Transformation|SetRelativeRotation (Variables|/Game/Excavator/ExcavatorSimulation_BP/BP_UpperArm.BP_UpperArm_C|GetBoom%20Pivot _asbp_upper_arm) "0, 0, 0" false false))

(event EventBeginPlay)

(event Collision|EventActorBeginOverlap
  (params (OtherActor :type Actor%20Object%20Reference)))

(event EventTick
  (params (DeltaSeconds :type Float%20%28single-precision%29)))

(event EventCollision?
  (params (Quest_Index :type Integer))
  (Class|BlackboardComponent|SetValueasInt (AI|GetBlackboard (AI|GetAIController (Actor|GetParentActor (Actor|GetParentActor)))) (Variables|Default|GetQuest_Number) Quest_Index)
  (CallFunction|CreateRock))

(fn ConstructionScript)