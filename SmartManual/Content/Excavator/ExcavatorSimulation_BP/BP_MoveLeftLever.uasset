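; Left travel lever actor for the excavator, driving its parent actor forward or backward.
; Up and Down events mark a drag, call MoveFront or MoveBack on Excavator_Simulation and tilt the Arrow component.
; Tick nudges the Arrow back based on world roll while not dragging.
; Separate functions, uncalled here, play front/back sequences and set left-side movement flags on either Excavator_Explain or Excavator_Simulation.
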(event EventBeginPlay
  ;[0.15 0.15 0.15 0.5] 이벤트 바인딩
  (Input|EnableInput 0))

(event Collision|EventActorBeginOverlap
  (params (OtherActor :type Actor%20Object%20Reference)))

(event EventTick
  (params (DeltaSeconds :type Float%20%28single-precision%29))
  (if (not (Variables|Default|GetDrag?))
    (CallFunction|ResetUpDownLever)))

(event EventDragComplete
  (Variables|Default|SetDrag? false))

(event EventDown
  (params (BT :type Object%20Object%20Reference))
  (Variables|Default|SetDrag? true)
  (CallFunction|Back))

(event EventUp
  (params (BT :type Object%20Object%20Reference))
  (Variables|Default|SetDrag? true)
  (CallFunction|Front))

(fn ConstructionScript)

(fn PlayFrontSequence
  (bind _returnvalue (Actor|GetParentActor))
  (Class|ActorSequenceComponent|PlaySequence (Variables|Default|GetFrontSequence))
  (bind _asexcavator_explain (Utilities|Casting|CastToExcavator_Explain _returnvalue)
    (:then
      (Variables|/Game/Excavator/Excavator_Explain.Excavator_Explain_C|SetGoStraight_Left? _asexcavator_explain true))
    (:CastFailed
      (bind _asexcavator_simulation (Utilities|Casting|CastToExcavator_Simulation _returnvalue))
      (Variables|/Game/Excavator/Excavator_Simulation.Excavator_Simulation_C|SetGoStraight_Left? _asexcavator_simulation true))))

(fn PlayBackSequence
  (bind _returnvalue (Actor|GetParentActor))
  (Class|ActorSequenceComponent|PlaySequence (Variables|Default|GetBackSequence))
  (bind _asexcavator_explain (Utilities|Casting|CastToExcavator_Explain _returnvalue)
    (:then
      (Variables|/Game/Excavator/Excavator_Explain.Excavator_Explain_C|SetGoBack_Left? _asexcavator_explain true))
    (:CastFailed
      (bind _asexcavator_simulation (Utilities|Casting|CastToExcavator_Simulation _returnvalue))
      (Variables|/Game/Excavator/Excavator_Simulation.Excavator_Simulation_C|SetGoBack_Left? _asexcavator_simulation true))))

(fn ResetUpDownLever
  (bind _arrow (Variables|Default|GetArrow))
  (bind _arrow_2 (Variables|Default|GetArrow))
  (bind _returnvalue (Transformation|GetWorldRotation _arrow))
  (if (!= (.roll (Transformation|GetWorldRotation (Variables|Default|GetArrow))) 0.0)
    (if (> (.roll _returnvalue) 0.0)
      (Transformation|AddRelativeRotation _arrow_2 "0.000000,0.000000,-0.300000" false false)
      (elif (< (.roll _returnvalue) 0.0)
        (Transformation|AddRelativeRotation _arrow_2 "0.000000,0.000000,0.300000" false false)))))

(fn Front
  (bind _arrow (Variables|Default|GetArrow))
  (bind _asexcavator_simulation (Utilities|Casting|CastToExcavator_Simulation (Actor|GetParentActor)))
  (Default|MoveFront _asexcavator_simulation)
  (if (<= (.pitch (Transformation|GetWorldRotation _arrow)) 2e+01)
    (Transformation|AddRelativeRotation _arrow "0.000000,0.000000,0.300000" false false)))

(fn Back
  (bind _arrow (Variables|Default|GetArrow))
  (bind _asexcavator_simulation (Utilities|Casting|CastToExcavator_Simulation (Actor|GetParentActor)))
  (Default|MoveBack _asexcavator_simulation)
  (if (<= (.pitch (Transformation|GetWorldRotation _arrow)) 2e+01)
    (Transformation|AddRelativeRotation _arrow "0.000000,0.000000,-0.300000" false false)))