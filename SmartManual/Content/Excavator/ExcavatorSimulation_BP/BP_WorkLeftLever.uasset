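; Left work lever of the excavator simulation, a child actor that swings the excavator and raises or lowers its boom.
; Left/Right events call turn functions on the parent Excavator_Simulation, while Up/Down rotate the BoomPivot of its BP_UpperArm child actor directly.
; Each input also tilts the lever's Arrow in small steps within a limited range.
; When not dragged, Tick steps the lever back toward neutral on both axes.
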(event EventBeginPlay
  ;[0.15 0.15 0.15 0.5] 이벤트 바인딩
  (Input|EnableInput 0))

(event Collision|EventActorBeginOverlap
  (params (OtherActor :type Actor%20Object%20Reference)))

(event EventLeft
  (params (BT :type Object%20Object%20Reference))
  (Variables|Default|SetDrag? true)
  (CallFunction|TurnLeft))

(event EventUp
  (params (BT :type Object%20Object%20Reference))
  (Variables|Default|SetDrag? true)
  (CallFunction|BoomDown))

(event EventDown
  (params (BT :type Object%20Object%20Reference))
  (Variables|Default|SetDrag? true)
  (CallFunction|BoomUp))

(event EventTick
  (params (DeltaSeconds :type Float%20%28single-precision%29))
  (if (not (Variables|Default|GetDrag?))
    (CallFunction|ResetUpDownLever)
    (CallFunction|ResetLeftRightLever)))

(event EventDragComplete
  (Variables|Default|SetDrag? false))

(event EventRight
  (params (BT :type Object%20Object%20Reference))
  (Variables|Default|SetDrag? true)
  (CallFunction|TurnRight))

(fn ConstructionScript)

(fn TurnLeft
  (bind _arrow (Variables|Default|GetArrow))
  (bind _asexcavator_simulation (Utilities|Casting|CastToExcavator_Simulation (Actor|GetParentActor)))
  (Default|TurnLeft _asexcavator_simulation)
  (if (<= (.pitch (Transformation|GetWorldRotation _arrow)) 2e+01)
    (Transformation|AddRelativeRotation _arrow "0.300000,0.000000,0.000000" false false)))

(fn ResetLeftRightLever
  (bind _arrow (Variables|Default|GetArrow))
  (bind _arrow_2 (Variables|Default|GetArrow))
  (bind _returnvalue (Transformation|GetWorldRotation _arrow))
  (if (!= (.pitch (Transformation|GetWorldRotation (Variables|Default|GetArrow))) 0.0)
    (if (> (.pitch _returnvalue) 0.0)
      (Transformation|AddRelativeRotation _arrow_2 "-0.300000,0.000000,0.000000" false false)
      (elif (< (.pitch _returnvalue) 0.0)
        (Transformation|AddRelativeRotation _arrow_2 "0.300000,0.000000,0.000000" false false)))))

(fn TurnRight
  (bind _arrow (Variables|Default|GetArrow))
  (bind _asexcavator_simulation (Utilities|Casting|CastToExcavator_Simulation (Actor|GetParentActor)))
  (Default|TurnRight _asexcavator_simulation)
  (if (>= (.pitch (Transformation|GetWorldRotation _arrow)) -2e+01)
    (Transformation|AddRelativeRotation _arrow "-0.300000,0.000000,0.000000" false false)))

(fn BoomDown
  (bind _arrow (Variables|Default|GetArrow))
  (bind _asexcavator_simulation (Utilities|Casting|CastToExcavator_Simulation (Actor|GetParentActor)))
  (bind _asbp_upper_arm (Utilities|Casting|CastToBP_UpperArm (Variables|/Script/Engine.ChildActorComponent|GetChildActor (Variables|/Game/Excavator/Excavator_Simulation.Excavator_Simulation_C|GetBoom%20Arm%20Basket _asexcavator_simulation))))
  (Transformation|AddRelativeRotation (Variables|/Game/Excavator/ExcavatorSimulation_BP/BP_UpperArm.BP_UpperArm_C|GetBoom%20Pivot _asbp_upper_arm) "0.000000,0.000000,-0.300000" false false)
  (if (<= (.roll (Transformation|GetWorldRotation _arrow)) 2e+01)
    (Transformation|AddRelativeRotation _arrow "0.000000,0.000000,0.300000" false false)))

(fn BoomUp
  (bind _arrow (Variables|Default|GetArrow))
  (bind _asexcavator_simulation (Utilities|Casting|CastToExcavator_Simulation (Actor|GetParentActor)))
  (bind _asbp_upper_arm (Utilities|Casting|CastToBP_UpperArm (Variables|/Script/Engine.ChildActorComponent|GetChildActor (Variables|/Game/Excavator/Excavator_Simulation.Excavator_Simulation_C|GetBoom%20Arm%20Basket _asexcavator_simulation))))
  (Transformation|AddRelativeRotation (Variables|/Game/Excavator/ExcavatorSimulation_BP/BP_UpperArm.BP_UpperArm_C|GetBoom%20Pivot _asbp_upper_arm) "0.000000,0.000000,0.300000" false false)
  (if (>= (.roll (Transformation|GetWorldRotation _arrow)) -2e+01)
    (Transformation|AddRelativeRotation _arrow "0.000000,0.000000,-0.300000" false false)))

(fn ResetUpDownLever
  (bind _arrow (Variables|Default|GetArrow))
  (bind _arrow_2 (Variables|Default|GetArrow))
  (bind _returnvalue (Transformation|GetWorldRotation _arrow))
  (if (!= (.roll (Transformation|GetWorldRotation (Variables|Default|GetArrow))) 0.0)
    (if (> (.roll _returnvalue) 0.0)
      (Transformation|AddRelativeRotation _arrow_2 "0.000000,0.000000,-0.300000" false false)
      (elif (< (.roll _returnvalue) 0.0)
        (Transformation|AddRelativeRotation _arrow_2 "0.000000,0.000000,0.300000" false false)))))