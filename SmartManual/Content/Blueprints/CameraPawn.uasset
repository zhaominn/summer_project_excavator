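; Player camera pawn for an excavator explainer that turns mouse drags on actors into directional commands.
; BeginPlay shows explain and skip widgets and blends the view to the Excavator_Explain actor; UpdateExplain forwards text to the explain widget.
; Clicking traces the actor under the cursor; release sends it Left/Right/Up/Down messages by dominant drag axis, with upward drags sending Down.
; Mid-drag direction checks, gated by Simulation, only print debug strings.
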(event Input|EnhancedActionEvents|EnhancedInputActionIA_MouseClick
  (params (ActionValue :type Boolean) (ElapsedSeconds :type Float%20%28double-precision%29) (TriggeredSeconds :type Float%20%28double-precision%29) (InputAction :type Input%20Action%20Object%20Reference :default "/Game/Input/IA_MouseClick.IA_MouseClick"))
  (:Triggered
    (CallFunction|MouseDragStart ActionValue)
    (Variables|Default|Setstart%20time TriggeredSeconds)
    (Variables|Default|SetDrag? true))
  (:Completed
    (CallFunction|MouseDragEnd)
    (Variables|Default|SetDrag? false)))

(event Input|EnhancedActionEvents|EnhancedInputActionIA_MouseMove
  (params (ActionValue :type Vector%202D%20Structure) (ElapsedSeconds :type Float%20%28double-precision%29) (TriggeredSeconds :type Float%20%28double-precision%29) (InputAction :type Input%20Action%20Object%20Reference :default "/Game/Input/IA_MouseMove.IA_MouseMove"))
  (bind _returnvalue (Game|GetPlayerController 0))
  (bind _startposition (Variables|Default|GetStartPosition))
  (bind (_locationx _locationy) (Game|Player|GetMousePosition _returnvalue))
  (if (Variables|Default|GetDrag?)
    (if (Variables|Default|GetSimulation?)
      (if (>= (- (Utilities|Time|GetTimeSeconds) (Variables|Default|Getstart%20time)) 1.0)
        (Variables|Default|Setstart%20time (Utilities|Time|GetTimeSeconds))
        (bind _output_get (Variables|Default|SetEndPosition (Math|Vector2D|MakeVector2D _locationx _locationy)))
        (if (> (Math|Float|Absolute(Float) (.x (- _output_get (Variables|Default|GetStartPosition)))) (Math|Float|Absolute(Float) (.y (- _output_get (Variables|Default|GetStartPosition)))))
          (if (< (.x (Variables|Default|GetEndPosition)) (.x _startposition))
            (Development|PrintString "좌")
            (else
              (Development|PrintString "우")))
          (elif (< (.y (Variables|Default|GetEndPosition)) (.y _startposition))
            (Development|PrintString "상")
            (else
              (Development|PrintString "하"))))))))

(event EventBeginPlay
  (bind _returnvalue (UserInterface|CreateWidget "/Game/UI/Explain/Explain_Widget.Explain_Widget_C"))
  (UserInterface|Viewport|AddtoViewport _returnvalue 0)
  (Variables|Default|Setexplain%20widget _returnvalue)
  (bind _returnvalue_2 (Actor|GetActorOfClass "/Game/Excavator/Excavator_Explain.Excavator_Explain_C"))
  (bind _output_get (Variables|Default|SetExcavator%20Ref _returnvalue_2))
  (Game|Player|SetViewTargetwithBlend (Game|GetPlayerController 0) _output_get 0.0 "VTBlend_Linear" 0.0 false)
  (bind _returnvalue_3 (UserInterface|CreateWidget "/Game/UI/WBP/WBP_Skip.WBP_Skip_C"))
  (UserInterface|Viewport|AddtoViewport _returnvalue_3 0))

(event Collision|EventActorBeginOverlap
  (params (OtherActor :type Actor%20Object%20Reference)))

(event EventTick
  (params (DeltaSeconds :type Float%20%28single-precision%29)))

(fn ConstructionScript)

(fn UpdateExplain
  (params (text :type Text))
  (Default|UpdateExplainText (Variables|Default|Getexplain%20widget) text))

(fn MouseDragStart
  (params (Condition :type Boolean))
  (bind _returnvalue (Game|GetPlayerController 0))
  (bind (_locationx _locationy) (Game|Player|GetMousePosition _returnvalue))
  (if Condition
    (Variables|Default|SetStartPosition (Math|Vector2D|MakeVector2D _locationx _locationy))
    (bind _output_get (Variables|Default|SetSelected%20Actor (.HitActor (Collision|BreakHitResult (.HitResult (Game|Player|GetHitResultUnderCursorbyChannel (Game|GetPlayerController 0) "TraceTypeQuery1" true))))))
    (Development|PrintText (Utilities|Text|ToText(Object) _output_get))))

(fn MouseDragEnd
  (bind _returnvalue (Game|GetPlayerController 0))
  (bind _selected_actor (Variables|Default|GetSelected%20Actor))
  (bind _startposition (Variables|Default|GetStartPosition))
  (bind (_locationx _locationy) (Game|Player|GetMousePosition _returnvalue))
  ;[0.15 0.15 0.15 0.5] end position
  (bind _output_get (Variables|Default|SetEndPosition (Math|Vector2D|MakeVector2D _locationx _locationy)))
  (if (> (Math|Float|Absolute(Float) (.x (- _output_get (Variables|Default|GetStartPosition)))) (Math|Float|Absolute(Float) (.y (- _output_get (Variables|Default|GetStartPosition)))))
    (if (< (.x (Variables|Default|GetEndPosition)) (.x _startposition))
      (Class|ComponentInterface|Left(Message) _selected_actor _selected_actor)
      (else
        (Class|ComponentInterface|Right(Message) _selected_actor _selected_actor)))
    (elif (< (.y (Variables|Default|GetEndPosition)) (.y _startposition))
      (Class|ComponentInterface|Down(Message) _selected_actor _selected_actor)
      (else
        (Class|ComponentInterface|Up(Message) _selected_actor _selected_actor)))))