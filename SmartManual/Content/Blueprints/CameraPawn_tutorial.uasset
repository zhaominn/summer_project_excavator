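; Tutorial camera pawn that shows an explanation widget, views through the Excavator_Tutorial actor and turns mouse drags into directional messages.
; Mouse click records the cursor position and selects the actor under it by trace.
; The dominant drag axis picks Left, Right, Up or Down, with screen-up sending Down, on release and on Tick while Simulation and Drag are true.
; Release also sends DragCompleteMessage; UpdateExplain updates the widget text.
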(event Input|EnhancedActionEvents|EnhancedInputActionIA_MouseClick
  (params (ActionValue :type Boolean) (ElapsedSeconds :type Float%20%28double-precision%29) (TriggeredSeconds :type Float%20%28double-precision%29) (InputAction :type Input%20Action%20Object%20Reference :default "/Game/Input/IA_MouseClick.IA_MouseClick"))
  (:Triggered
    (CallFunction|MouseDragStart ActionValue)
    (Variables|Default|SetDrag? true))
  (:Completed
    (CallFunction|MouseDragEnd)
    (Class|ComponentInterface|DragComplete(Message) (Variables|Default|GetSelected%20Actor))
    (Variables|Default|SetDrag? false)))

(event EventBeginPlay
  (bind _returnvalue (UserInterface|CreateWidget "/Game/UI/Explain/Explain_Widget.Explain_Widget_C"))
  (UserInterface|Viewport|AddtoViewport _returnvalue 0)
  (Variables|Default|Setexplain%20widget _returnvalue)
  (bind _returnvalue_2 (Actor|GetActorOfClass "/Game/Excavator/Excavator_Tutorial.Excavator_Tutorial_C"))
  (bind _output_get (Variables|Default|SetNewVar _returnvalue_2))
  (Game|Player|SetViewTargetwithBlend (Game|GetPlayerController 0) _output_get 0.0 "VTBlend_Linear" 0.0 false))

(event Collision|EventActorBeginOverlap
  (params (OtherActor :type Actor%20Object%20Reference)))

(event EventTick
  (params (DeltaSeconds :type Float%20%28single-precision%29))
  (bind _returnvalue (Game|GetPlayerController 0))
  (bind _selected_actor (Variables|Default|GetSelected%20Actor))
  (bind _startposition (Variables|Default|GetStartPosition))
  (bind (_locationx _locationy) (Game|Player|GetMousePosition _returnvalue))
  (if (and (Variables|Default|GetSimulation?) (Variables|Default|GetDrag?))
    (if (>= (- (Utilities|Time|GetTimeSeconds) 0.0) 0.05)
      (bind _output_get (Variables|Default|SetEndPosition (Math|Vector2D|MakeVector2D _locationx _locationy)))
      (if (> (Math|Float|Absolute(Float) (.x (- _output_get (Variables|Default|GetStartPosition)))) (Math|Float|Absolute(Float) (.y (- _output_get (Variables|Default|GetStartPosition)))))
        (if (< (.x (Variables|Default|GetEndPosition)) (.x _startposition))
          (Development|PrintString "좌")
          (Class|ComponentInterface|Left(Message) _selected_actor _selected_actor)
          (else
            (Development|PrintString "우")
            (Class|ComponentInterface|Right(Message) _selected_actor _selected_actor)))
        (elif (< (.y (Variables|Default|GetEndPosition)) (.y _startposition))
          (Development|PrintString "상")
          (Class|ComponentInterface|Down(Message) _selected_actor _selected_actor)
          (else
            (Development|PrintString "하")
            (Class|ComponentInterface|Up(Message) _selected_actor _selected_actor)))))))

(fn ConstructionScript)

(fn UpdateExplain
  (params (text :type Text))
  (Default|UpdateExplainText (Variables|Default|Getexplain%20widget) text))

(fn MouseDragStart
  (params (Condition :type Boolean))
  (bind _returnvalue (Game|GetPlayerController 0))
  (bind (_locationx _locationy) (Game|Player|GetMousePosition _returnvalue))
  (if Condition
    (Variables|Default|SetStartPosition (Math|Vector2D|MakeVector2D _locationx _locationy))
    (Variables|Default|SetSelected%20Actor (.HitActor (Collision|BreakHitResult (.HitResult (Game|Player|GetHitResultUnderCursorbyChannel (Game|GetPlayerController 0) "TraceTypeQuery1" true)))))))

(fn MouseDragEnd
  (bind _returnvalue (Game|GetPlayerController 0))
  (bind _selected_actor (Variables|Default|GetSelected%20Actor))
  (bind _startposition (Variables|Default|GetStartPosition))
  (bind (_locationx _locationy) (Game|Player|GetMousePosition _returnvalue))
  ;[0.15 0.15 0.15 0.5] end position
  (bind _output_get (Variables|Default|SetEndPosition (Math|Vector2D|MakeVector2D _locationx _locationy)))
  (if (> (Math|Float|Absolute(Float) (.x (- _output_get (Variables|Default|GetStartPosition)))) (Math|Float|Absolute(Float) (.y (- _output_get (Variables|Default|GetStartPosition)))))
    (if (< (.x (Variables|Default|GetEndPosition)) (.x _startposition))
      (Class|ComponentInterface|Left(Message) _selected_actor _selected_actor)
      (else
        (Class|ComponentInterface|Right(Message) _selected_actor _selected_actor)))
    (elif (< (.y (Variables|Default|GetEndPosition)) (.y _startposition))
      (Class|ComponentInterface|Down(Message) _selected_actor _selected_actor)
      (else
        (Class|ComponentInterface|Up(Message) _selected_actor _selected_actor)))))