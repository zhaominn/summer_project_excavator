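; BP_Instance is a game instance that handles level switching by index.
; ChangeLevel prints the current level index, clamps it to a fixed range, then loops through LevelArray to open the level name stored at that index.
; Init only prints a debug message when the instance starts.
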(event Custom|ChangeLevel
  ;[0.15 0.15 0.15 0.5] change map
  (Development|PrintString (Utilities|String|ToString(Integer) (Variables|Default|GetCurrentLevelIndex)))
  (Variables|Default|SetCurrentLevelIndex (Math|Integer|Clamp(Integer) (Variables|Default|GetCurrentLevelIndex) 0 20))
  (for (_array_element _array_index) (Variables|Default|GetLevelArray)
    (if (== _array_index (Variables|Default|GetCurrentLevelIndex))
      (Game|OpenLevel(byName) _array_element))))

(event EventInit
  (Development|PrintString "instance 시작"))